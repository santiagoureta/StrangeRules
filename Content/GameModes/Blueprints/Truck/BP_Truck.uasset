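; Truck vehicle Blueprint that drives itself along a road spline.
; Each tick it gets the road spline, computes steering via GetPath, prints that value, and applies it with a constant throttle.
; GetPath projects a look-ahead point along the nearest spline tangent, snaps it back onto the spline, and maps the yaw difference toward it to a clamped steering input.
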(event `self.ReceiveTick`
  (params (DeltaSeconds :type "Float (single-precision)"))
  (bind _vehiclemovementcomponent (`self.VehicleMovementComponent`))
  (bind _returnvalue (`self.GetRoadSpline`))
  (if (`KismetSystemLibrary.IsValid` _returnvalue)
    (bind _steering (`self.GetPath` _returnvalue))
    (`KismetSystemLibrary.PrintString` (`KismetStringLibrary.Conv_DoubleToString` _steering))
    (`ChaosVehicleMovementComponent.SetSteeringInput` _vehiclemovementcomponent _steering)
    (`ChaosVehicleMovementComponent.SetThrottleInput` _vehiclemovementcomponent 0.8)))

(fn `GetPath`
  (params (Spline :type "SplineComponent Object Reference"))
  (returns (Steering :type "Float (double-precision)"))
  (bind _returnvalue (`self.K2_GetActorLocation`))
  (bind (_returnvalue_roll _returnvalue_pitch _returnvalue_yaw) (`KismetMathLibrary.BreakRotator` (`KismetMathLibrary.NormalizedDeltaRotator` (`KismetMathLibrary.FindLookAtRotation` _returnvalue (`SplineComponent.FindLocationClosestToWorldLocation` Spline (+ (* (`KismetMathLibrary.Normal` (`SplineComponent.FindTangentClosestToWorldLocation` Spline _returnvalue "World")) 500.0) _returnvalue) "World")) (`self.K2_GetActorRotation`))))
  (return (`KismetMathLibrary.MapRangeClamped` _returnvalue_yaw 45.0 -45.0 1.0 -1.0)))

(fn `UserConstructionScript`)